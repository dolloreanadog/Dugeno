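; Game instance for Flighter that holds the player's lives and handles level flow.
; On player death it decrements and prints Lives and reloads the current level by name, or opens the bad-ending menu when none remain.
; Collecting the maximum capsules opens the good-ending menu, and Escape opens the main menu.
; Init and OnCapsuleCollected are empty stubs.
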(event Custom|OnPlayerDies
  (if (<= (Variables|Default|GetLives) 0)
    (Game|OpenLevel(byObjectReference) "/Game/Maps/GameMenu_Bad.GameMenu_Bad")
    (else
      (bind _result (Math|Integer|DecrementInt (Variables|Default|GetLives))
        (:%20%20
          (Development|PrintString (Utilities|String|ToString(Integer) _result))
          (CallFunction|RestartLevel))))))

(event Custom|OnMaxCapsulesCollected
  (Game|OpenLevel(byObjectReference) "/Game/Maps/GameMenu_Good.GameMenu_Good"))

(event Custom|OnPressEscape
  (Game|OpenLevel(byObjectReference) "/Game/Maps/GameMenu.GameMenu"))

(event EventInit)

(fn RestartLevel
  (bind _returnvalue (Game|GetCurrentLevelName true))
  (Game|OpenLevel(byName) (Utilities|String|StringToName _returnvalue)))

(fn OnCapsuleCollected)