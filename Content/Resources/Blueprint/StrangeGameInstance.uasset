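; StrangeGameInstance is the game instance that tracks difficulty, battle count and turn count for the game's battles.
; An enemy death raises difficulty and opens the Plinko level, while a friend death lowers it; values at zero or below reset to one.
; NextTurn increments the turn counter and removes a turn from the BasicAttackEffect component on the Bow actor, if one exists.
; ChangeLevel is an empty stub.
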(event Custom|EnemyDies
  (CallFunction|AddDifficulty 1)
  (Game|OpenLevel(byObjectReference) "/Game/Resources/Maps/GameMaps/Plinko.Plinko"))

(event Custom|FriendDies
  (CallFunction|AddDifficulty -1))

(event Custom|ChangeLevel)

(event Custom|NextBattle
  (Variables|Default|SetNumberOfBattles (+ (Variables|Default|GetNumberOfBattles) 1))
  (CallFunction|AddDifficulty))

(event EventInit
  (bind _returnvalue (Game|GetCurrentLevelName true))
  (Development|PrintString _returnvalue))

(fn AddDifficulty
  (params (ChangeBy :type Integer))
  (Variables|Default|SetDifficulty (+ (Variables|Default|GetDifficulty) ChangeBy))
  (if (<= (Variables|Default|GetDifficulty) 0)
    (bind _output_get (Variables|Default|SetDifficulty 1))
    (Development|PrintString (Utilities|String|ToString(Integer) _output_get))))

(fn NextTurn
  (Variables|Default|SetNumberOfTurns (+ (Variables|Default|GetNumberOfTurns) 1))
  (bind _returnvalue (Actor|GetActorOfClass "/Game/Resources/Characters/Bow/Bow.Bow_C"))
  (Utilities|IsValid (Actor|GetComponentbyClass _returnvalue "/Game/Resources/Components/StatusEffects/BasicAttackEffect.BasicAttackEffect_C")
    (:Is%20Valid
      (Default|RemoveTurn (Actor|GetComponentbyClass _returnvalue "/Game/Resources/Components/StatusEffects/BasicAttackEffect.BasicAttackEffect_C"))
      (Development|PrintString "Turn End"))
    (:Is%20Not%20Valid
      (Development|PrintString "No Longer Exist"))))